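; Battle Royale controller for a Mordhau mod that arms spawned characters with a platform gun.
; On character spawn it waits briefly, then, if the Battle Royale game mode has initialized the match, spawns the gun and puts it in the character's first slot.
; A ParryThis event applies a replicated health loss to the controlled character.
; Console log messages trace startup, spawning and the gun handout.
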(event EventBeginPlay
  (|CallParentFunction)
  (Utilities|FlowControl|Delay 1.0)
  (Class|MordhauUtilityLibrary|PrinttoConsoleandLog "Character started" false))

(event EventTick
  (params (DeltaSeconds :type Float%20%28single-precision%29))
  (|CallParentFunction DeltaSeconds) ; This node is disabled and will not be called.\nDrag off pins to build functionality.
)

(event EventOnMordhauCharacterSpawned
  (params (SpawnedCharacter :type Mordhau%20Character%20Object%20Reference))
  (|CallParentFunction SpawnedCharacter)
  (Class|MordhauUtilityLibrary|PrinttoConsoleandLog "CharacterSpawned" false)
  (Utilities|FlowControl|Delay 1.0)
  (bind _asbp_battle_royale_game_mode (Utilities|Casting|CastToBP_BattleRoyaleGameMode (Game|GetGameMode)))
  (if (Variables|/Game/Mordhau/Blueprints/GameModes/BattleRoyale/BP_BattleRoyaleGameMode.BP_BattleRoyaleGameMode_C|GetInitializedMatch _asbp_battle_royale_game_mode)
    (bind _returnvalue (Game|SpawnActorfromClass "/RandomWeapon_BattleRoyal/Weapons/BuildingGuns/BP_PlatformGun.BP_PlatformGun_C" (Transformation|GetActorTransform SpawnedCharacter) "AlwaysSpawn" SpawnedCharacter 0))
    (Class|MordhauCharacter|PickUptoSlot SpawnedCharacter _returnvalue)
    (Class|MordhauUtilityLibrary|PrinttoConsoleandLog "gun given" false)))

(event EventParryThis
  (bind _asbp_mordhau_character (Utilities|Casting|CastToBP_MordhauCharacter (Pawn|GetControlledPawn)))
  (Class|AdvancedCharacter|OffsetHealth _asbp_mordhau_character -100 true))

(fn ConstructionScript
  (|CallParentFunction))