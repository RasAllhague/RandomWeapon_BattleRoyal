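; BP_KickWeaponPickup is a weapon-style pickup that upgrades the owning character's kick weapon.
; When its attack starts, it runs the parent logic, then spawns an UpgradedKick actor at the current kick weapon's transform, owned by the character.
; The new actor replaces the character's KickWeapon reference, with no destroy call on the previous weapon here.
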(event EventBeginPlay
  (|CallParentFunction) ; This node is disabled and will not be called.\nDrag off pins to build functionality.
)

(event Collision|EventActorBeginOverlap
  (params (OtherActor :type Actor%20Object%20Reference))
  (|CallParentFunction OtherActor) ; This node is disabled and will not be called.\nDrag off pins to build functionality.
)

(event EventTick
  (params (DeltaSeconds :type Float%20%28single-precision%29))
  (|CallParentFunction DeltaSeconds) ; This node is disabled and will not be called.\nDrag off pins to build functionality.
)

(event EventOnAttackStarted
  (params (Move :type EAttackMove%20Enum :default "RightStrike") (Angle :type Float%20%28single-precision%29))
  (bind _returnvalue (Class|MordhauEquipment|GetParentCharacter))
  (|CallParentFunction Move Angle)
  (bind _returnvalue_2 (Game|SpawnActorfromClass (Variables|Default|GetUpgradedKick) (Transformation|GetActorTransform (Variables|/Script/Mordhau.MordhauCharacter|GetKickWeapon _returnvalue)) "Undefined" _returnvalue 0))
  (Variables|/Script/Mordhau.MordhauCharacter|SetKickWeapon _returnvalue _returnvalue_2))

(fn ConstructionScript
  (|CallParentFunction))