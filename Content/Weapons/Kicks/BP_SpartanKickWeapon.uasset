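; BP_SpartanKickWeapon is a kick weapon that sends a struck character flying in the direction the attacker is looking.
; After the parent OnHit logic runs, hits on a BP_MordhauCharacter call PushEnemy with a fixed-strength vector along the kicker's camera forward, pitch included.
; PushEnemy overwrites the target's CharacterMovement velocity directly rather than using LaunchCharacter or an impulse.
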(event Custom|PushEnemy
  (params (Player :type BP%20Mordhau%20Character%20Object%20Reference) (Velocity :type Vector))
  (Variables|/Script/Engine.MovementComponent|SetVelocity (Variables|/Script/Engine.Character|GetCharacterMovement Player) Velocity))

(event EventBeginPlay
  (|CallParentFunction) ; This node is disabled and will not be called.\nDrag off pins to build functionality.
)

(event Collision|EventActorBeginOverlap
  (params (OtherActor :type Actor%20Object%20Reference))
  (|CallParentFunction OtherActor) ; This node is disabled and will not be called.\nDrag off pins to build functionality.
)

(event EventTick
  (params (DeltaSeconds :type Float%20%28single-precision%29))
  (|CallParentFunction DeltaSeconds) ; This node is disabled and will not be called.\nDrag off pins to build functionality.
)

(event EventOnHit
  (params (Actor :type Actor%20Object%20Reference) (Move :type EAttackMove%20Enum :default "RightStrike") (Bone :type Name :default "None") (WorldLocation :type Vector%20%28by%20ref%29 :default "0, 0, 0") (Tier :type Byte :default 0) (SurfaceType :type Byte :default 0))
  (bind _returnvalue (Class|MordhauEquipment|GetParentCharacter))
  (bind _mordhaucamera (Variables|/Script/Mordhau.MordhauCharacter|GetMordhauCamera _returnvalue))
  (bind _returnvalue_2 (Transformation|GetWorldLocation _mordhaucamera))
  (|CallParentFunction Actor Move Bone WorldLocation Tier SurfaceType)
  (bind _asbp_mordhau_character (Utilities|Casting|CastToBP_MordhauCharacter Actor))
  (CallFunction|PushEnemy _asbp_mordhau_character (* (Math|Vector|GetUnitDirection(Vector) _returnvalue_2 (+ _returnvalue_2 (* (Math|Vector|GetForwardVector (Transformation|GetWorldRotation _mordhaucamera)) 1e+03))) 2.5e+03)))

(fn ConstructionScript
  (|CallParentFunction))