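; Mordhau sword weapon Blueprint that gives its wielder a force push on the T key, available only outside of attacks.
; Tick polls the player controller for the key, plays a yield montage and yell, then box-traces pawns along the camera's forward direction.
; Each character hit has its velocity overwritten along that direction and is tripped.
; Debug prints and trace drawing remain active.
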(event Custom|Force%20Push
  (params (pawn :type BP%20Mordhau%20Character%20Object%20Reference) (velocity :type Vector))
  (Development|PrintString "Casted it")
  (bind _output_get (Variables|/Script/Engine.MovementComponent|SetVelocity (Variables|/Script/Engine.Character|GetCharacterMovement pawn) velocity))
  (Development|PrintString (Utilities|String|ToString(Vector) _output_get))
  (Class|AdvancedCharacter|RequestTrip pawn)
  (Development|PrintString "Requested Trip"))

(event Custom|Push%20Animation
  (params (player :type BP%20Mordhau%20Character%20Object%20Reference))
  (Class|AdvancedCharacter|PlayAnim player "/Game/Mordhau/Animations/RawClips/Misc/Emotes/Throatcut1/MTG_Yield1.MTG_Yield1" 1.0 true)
  (Class|MordhauCharacter|PlayAttackYell player))

(event EventBeginPlay
  (|CallParentFunction) ; This node is disabled and will not be called.\nDrag off pins to build functionality.
)

(event Collision|EventActorBeginOverlap
  (params (OtherActor :type Actor%20Object%20Reference))
  (|CallParentFunction OtherActor) ; This node is disabled and will not be called.\nDrag off pins to build functionality.
)

(event EventTick
  (params (DeltaSeconds :type Float%20%28single-precision%29))
  (bind _returnvalue (Class|MordhauEquipment|GetParentCharacter))
  (bind _returnvalue_2 (Class|MordhauEquipment|GetParentCharacter))
  (bind _mordhaucamera (Variables|/Script/Mordhau.MordhauCharacter|GetMordhauCamera _returnvalue))
  (bind _returnvalue_3 (Transformation|GetWorldLocation _mordhaucamera))
  (bind _returnvalue_4 (Transformation|GetWorldRotation _mordhaucamera))
  (bind _returnvalue_5 (Math|Vector|GetForwardVector _returnvalue_4))
  (bind _returnvalue_6 (* _returnvalue_5 1e+03))
  (bind _returnvalue_7 (+ _returnvalue_3 _returnvalue_6))
  (|CallParentFunction DeltaSeconds)
  (if (Class|MordhauEquipment|BelongstoCharacter)
    (if (Variables|Default|GetCanUseForcePush)
      (bind _asbp_mordhau_player_controller (Utilities|Casting|CastToBP_MordhauPlayerController (Pawn|GetController _returnvalue_2)))
      (if (Game|Player|WasInputKeyJustPressed _asbp_mordhau_player_controller "T")
        (bind _asbp_mordhau_character (Utilities|Casting|CastToBP_MordhauCharacter _returnvalue_2)
          (:then
            (CallFunction|PushAnimation _asbp_mordhau_character)
            (bind (_outhits _returnvalue_8) (Class|KismetSystemLibrary|BoxTraceMultiforObjects _returnvalue_3 _returnvalue_7 "200.000000,200.000000,200.000000" _returnvalue_4 (Utilities|Array|MakeArray "ObjectTypeQuery3") false (Utilities|Array|MakeArray _returnvalue) "ForOneFrame" false))
            (Development|PrintString (Utilities|String|ToString(Boolean) _returnvalue_8))
            (for _array_element _outhits
              (bind _asbp_mordhau_character_2 (Utilities|Casting|CastToBP_MordhauCharacter (.HitActor (Collision|BreakHitResult _array_element))))
              (CallFunction|ForcePush _asbp_mordhau_character_2 (* (Math|Vector|GetUnitDirection(Vector) _returnvalue_3 _returnvalue_7) 2.5e+03))))
          (:CastFailed
            (Development|PrintString "SecondCast failed")))))))

(event EventOnAttackStarted
  (params (Move :type EAttackMove%20Enum :default "RightStrike") (Angle :type Float%20%28single-precision%29))
  (|CallParentFunction Move Angle)
  (Variables|Default|SetCanUseForcePush false))

(event EventOnAttackStopped
  (|CallParentFunction)
  (Variables|Default|SetCanUseForcePush true))

(fn ConstructionScript
  (|CallParentFunction))