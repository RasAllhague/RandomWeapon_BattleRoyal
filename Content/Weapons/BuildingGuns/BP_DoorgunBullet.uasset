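; Projectile fired by a building gun that places an actor where it lands, by its name a door.
; On hit, it resolves the owning Mordhau controller's last controlled character and the BP_BuildingGun that created it.
; It spawns ActorToSpawn at the hit location, taking yaw from the character and pitch from the gun's stepped rotation setting.
; That rotation is printed and reapplied after spawning; tick and overlap events are unused.
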(event EventBeginPlay
  (|CallParentFunction) ; This node is disabled and will not be called.\nDrag off pins to build functionality.
)

(event Collision|EventActorBeginOverlap
  (params (OtherActor :type Actor%20Object%20Reference))
  (|CallParentFunction OtherActor) ; This node is disabled and will not be called.\nDrag off pins to build functionality.
)

(event EventTick
  (params (DeltaSeconds :type Float%20%28single-precision%29))
  (|CallParentFunction DeltaSeconds) ; This node is disabled and will not be called.\nDrag off pins to build functionality.
)

(event EventOnProjectileHit
  (params (HitLocation :type Vector :default "0, 0, 0") (HitNormal :type Vector :default "0, 0, 0") (BounceForce :type Float%20%28single-precision%29) (Surface :type Byte :default 0) (bHasHitWorld :type Boolean) (bHasStopped :type Boolean))
  (|CallParentFunction HitLocation HitNormal BounceForce Surface bHasHitWorld bHasStopped)
  (bind _returnvalue (Class|MordhauProjectile|GetProjectileOwningController))
  (bind _asbp_mordhau_player_controller (Utilities|Casting|CastToBP_MordhauPlayerController _returnvalue))
  (bind _returnvalue_2 (Class|MordhauPlayerController|GetLastControlledCharacter _asbp_mordhau_player_controller))
  (bind _returnvalue_3 (Class|MordhauProjectile|GetProjectileCreator))
  (bind _asbp_building_gun (Utilities|Casting|CastToBP_BuildingGun _returnvalue_3))
  (Development|PrintString (Utilities|String|ToString(Rotator) (Math|Rotator|MakeRotator 0.0 (* (Variables|/RandomWeapon_BattleRoyal/Weapons/BuildingGuns/BP_BuildingGun.BP_BuildingGun_C|GetYRotInterval _asbp_building_gun) (Variables|/RandomWeapon_BattleRoyal/Weapons/BuildingGuns/BP_BuildingGun.BP_BuildingGun_C|GetYRotPerStep _asbp_building_gun)) (.Yaw (Math|Rotator|BreakRotator (Transformation|GetActorRotation _returnvalue_2))))))
  (bind _returnvalue_4 (Game|SpawnActorfromClass (Variables|Default|GetActorToSpawn) (Math|Transform|MakeTransform HitLocation (Math|Rotator|MakeRotator 0.0 (* (Variables|/RandomWeapon_BattleRoyal/Weapons/BuildingGuns/BP_BuildingGun.BP_BuildingGun_C|GetYRotInterval _asbp_building_gun) (Variables|/RandomWeapon_BattleRoyal/Weapons/BuildingGuns/BP_BuildingGun.BP_BuildingGun_C|GetYRotPerStep _asbp_building_gun)) (.Yaw (Math|Rotator|BreakRotator (Transformation|GetActorRotation _returnvalue_2))))) "Undefined" 0 0))
  (Transformation|SetActorRotation _returnvalue_4 (Math|Rotator|MakeRotator 0.0 (* (Variables|/RandomWeapon_BattleRoyal/Weapons/BuildingGuns/BP_BuildingGun.BP_BuildingGun_C|GetYRotInterval _asbp_building_gun) (Variables|/RandomWeapon_BattleRoyal/Weapons/BuildingGuns/BP_BuildingGun.BP_BuildingGun_C|GetYRotPerStep _asbp_building_gun)) (.Yaw (Math|Rotator|BreakRotator (Transformation|GetActorRotation _returnvalue_2)))) true))

(fn ConstructionScript
  (|CallParentFunction))