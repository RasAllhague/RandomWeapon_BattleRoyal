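; BP_BuildingGun is a Mordhau equipment Blueprint for a building gun, handling the Y-rotation setting and its display.
; While it belongs to a character, Tick polls that character's player controller for Q and E presses to step the rotation interval up or down.
; Each change calls UpdateName, which rebuilds the equipment name from the base name plus the resulting angle in parentheses.
; No placement or firing logic appears in this Blueprint.
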(event EventBeginPlay
  (|CallParentFunction) ; This node is disabled and will not be called.\nDrag off pins to build functionality.
)

(event Collision|EventActorBeginOverlap
  (params (OtherActor :type Actor%20Object%20Reference))
  (|CallParentFunction OtherActor) ; This node is disabled and will not be called.\nDrag off pins to build functionality.
)

(event EventTick
  (params (DeltaSeconds :type Float%20%28single-precision%29))
  (|CallParentFunction DeltaSeconds)
  (if (Class|MordhauEquipment|BelongstoCharacter)
    (bind _asbp_mordhau_player_controller (Utilities|Casting|CastToBP_MordhauPlayerController (Pawn|GetController (Class|MordhauEquipment|GetParentCharacter))))
    (if (Game|Player|WasInputKeyJustPressed _asbp_mordhau_player_controller "Q")
      (Variables|Default|SetYRotInterval (+ (Variables|Default|GetYRotInterval) 1))
      (CallFunction|UpdateName :!label _label)
      (elif (Game|Player|WasInputKeyJustPressed _asbp_mordhau_player_controller "E")
        (Variables|Default|SetYRotInterval (- (Variables|Default|GetYRotInterval) 1))
        (goto _label)))))

(fn ConstructionScript
  (|CallParentFunction))

(fn UpdateName
  (Variables|Default|SetEquipmentName (Utilities|Text|ToText(String) (Utilities|String|Append (Variables|Default|GetConcreteName) " (" (Utilities|String|ToString(Float) (* (Variables|Default|GetYRotInterval) (Variables|Default|GetYRotPerStep))) ")")))
  (return))