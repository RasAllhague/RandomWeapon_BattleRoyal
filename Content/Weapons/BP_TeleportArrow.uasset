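; BP_TeleportArrow is a projectile that teleports the pawn of the player who fired it to the point of impact.
; On each projectile hit it runs the parent logic, then casts the owning controller to BP_MordhauPlayerController and moves its controlled pawn to the hit location, keeping its rotation.
; Debug strings print the teleport result, or the controller's name when the cast fails.
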(event EventBeginPlay
  (|CallParentFunction) ; This node is disabled and will not be called.\nDrag off pins to build functionality.
)

(event Collision|EventActorBeginOverlap
  (params (OtherActor :type Actor%20Object%20Reference))
  (|CallParentFunction OtherActor) ; This node is disabled and will not be called.\nDrag off pins to build functionality.
)

(event EventTick
  (params (DeltaSeconds :type Float%20%28single-precision%29))
  (|CallParentFunction DeltaSeconds) ; This node is disabled and will not be called.\nDrag off pins to build functionality.
)

(event EventOnProjectileHit
  (params (HitLocation :type Vector :default "0, 0, 0") (HitNormal :type Vector :default "0, 0, 0") (BounceForce :type Float%20%28single-precision%29) (Surface :type Byte :default 0) (bHasHitWorld :type Boolean) (bHasStopped :type Boolean))
  (|CallParentFunction HitLocation HitNormal BounceForce Surface bHasHitWorld bHasStopped)
  (bind _returnvalue (Class|MordhauProjectile|GetProjectileOwningController))
  (bind _asbp_mordhau_player_controller (Utilities|Casting|CastToBP_MordhauPlayerController _returnvalue)
    (:then
      (bind _returnvalue_2 (Transformation|Teleport (Pawn|GetControlledPawn _asbp_mordhau_player_controller) HitLocation (Transformation|GetActorRotation (Pawn|GetControlledPawn _asbp_mordhau_player_controller))))
      (Development|PrintString (Utilities|String|ToString(Boolean) _returnvalue_2)))
    (:CastFailed
      (Development|PrintString (Utilities|GetDisplayName _asbp_mordhau_player_controller)))))

(fn ConstructionScript
  (|CallParentFunction))