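; BP_CarrotRain is a weapon Blueprint that spawns a BP_CarrotRainSpawner actor when it registers a hit.
; Its OnHit override runs the parent logic, then places the spawner at the hit location with a small offset along world X.
; The rain behavior itself is not in this graph, and BeginPlay, overlap and Tick are unused.
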(event EventBeginPlay
  (|CallParentFunction) ; This node is disabled and will not be called.\nDrag off pins to build functionality.
)

(event Collision|EventActorBeginOverlap
  (params (OtherActor :type Actor%20Object%20Reference))
  (|CallParentFunction OtherActor) ; This node is disabled and will not be called.\nDrag off pins to build functionality.
)

(event EventTick
  (params (DeltaSeconds :type Float%20%28single-precision%29))
  (|CallParentFunction DeltaSeconds) ; This node is disabled and will not be called.\nDrag off pins to build functionality.
)

(event EventOnHit
  (params (Actor :type Actor%20Object%20Reference) (Move :type EAttackMove%20Enum :default "RightStrike") (Bone :type Name :default "None") (WorldLocation :type Vector%20%28by%20ref%29 :default "0, 0, 0") (Tier :type Byte :default 0) (SurfaceType :type Byte :default 0))
  (bind (_x _y _z) (Math|Vector|BreakVector WorldLocation))
  (|CallParentFunction Actor Move Bone WorldLocation Tier SurfaceType)
  (Game|SpawnActorfromClass "/RandomWeapon_BattleRoyal/Weapons/BP_CarrotRainSpawner.BP_CarrotRainSpawner_C" (Math|Conversions|ToTransform(Vector) (Math|Vector|MakeVector (+ _x 1e+01) _y _z)) "Undefined" 0 0))

(fn ConstructionScript
  (|CallParentFunction))