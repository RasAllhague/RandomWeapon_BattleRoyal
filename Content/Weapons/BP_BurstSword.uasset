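; Mordhau sword weapon that earns a radial "Force Burst" shockwave through landed hits.
; OnHit counts hits while the burst is uncharged and arms it on the fifth, resetting the counter.
; Tick polls the owning player controller for the R key, then plays a first- or third-person shockwave montage and spends the charge.
; The burst deals falloff damage with knockback and ragdoll around the wielder, sparing friendlies.
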(event EventBeginPlay
  (|CallParentFunction) ; This node is disabled and will not be called.\nDrag off pins to build functionality.
)

(event Collision|EventActorBeginOverlap
  (params (OtherActor :type Actor%20Object%20Reference))
  (|CallParentFunction OtherActor) ; This node is disabled and will not be called.\nDrag off pins to build functionality.
)

(event EventTick
  (params (DeltaSeconds :type Float%20%28single-precision%29))
  (bind _returnvalue (Class|MordhauEquipment|GetParentCharacter))
  (|CallParentFunction DeltaSeconds)
  (if (Class|MordhauEquipment|BelongstoCharacter)
    (bind _asbp_mordhau_player_controller (Utilities|Casting|CastToBP_MordhauPlayerController (Pawn|GetController _returnvalue)))
    (if (and (Game|Player|WasInputKeyJustPressed _asbp_mordhau_player_controller "R") (Variables|Default|GetCanUseForce))
      (Class|AdvancedCharacter|PlayAnim _returnvalue (select (Variables|Default|GetbIsFirstPerson) "/Game/Mordhau/Animations/RawClips/Abilities/MTG_Shockwave_1P_V2.MTG_Shockwave_1P_V2" "/Game/Mordhau/Animations/RawClips/Abilities/MTG_Shockwave_V2.MTG_Shockwave_V2") 1.0 true)
      (Development|PrintString "Force Burst")
      (Variables|Default|SetCanUseForce false)
      (Class|MordhauUtilityLibrary|MordhauApplyRadialDamagewithFalloff 1e+01 5.0 0.0 0.0 (Transformation|GetActorLocation _returnvalue) 3e+02 4e+02 0.0 (Utilities|Array|MakeArray _returnvalue) 2.5e+03 1.5e+03 2e+02 _returnvalue 0 "ECC_Visibility" true))))

(event EventOnHit
  (params (Actor :type Actor%20Object%20Reference) (Move :type EAttackMove%20Enum :default "RightStrike") (Bone :type Name :default "None") (WorldLocation :type Vector%20%28by%20ref%29 :default "0, 0, 0") (Tier :type Byte :default 0) (SurfaceType :type Byte :default 0))
  (|CallParentFunction Actor Move Bone WorldLocation Tier SurfaceType)
  (if (not (Variables|Default|GetCanUseForce))
    (if (== (Variables|Default|Gethitcount) 4)
      (Variables|Default|SetCanUseForce true)
      (Variables|Default|Sethitcount 0)
      (else
        (Math|Integer|IncrementInt (Variables|Default|Gethitcount))))))

(fn ConstructionScript
  (|CallParentFunction))