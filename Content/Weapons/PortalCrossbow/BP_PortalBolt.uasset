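; Portal crossbow projectile that places one of two linked BP_SpecialPortal actors at its hit location.
; On hit, it finds the BP_PortalCrossbow in the shooter's equipment and reads its PortalSpawnMode.
; A missing portal is spawned with its type's material and cross-referenced with the crossbow; otherwise MovePortal teleports one.
; MovePortal selects the opposite slot to the requested type: First moves SecondPortal and vice versa.
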(event Custom|PortalShot
  (params (Transform :type Transform))
  (bind _returnvalue (Class|MordhauProjectile|GetProjectileOwningController))
  (bind _asbp_mordhau_player_controller (Utilities|Casting|CastToBP_MordhauPlayerController _returnvalue))
  (bind _array_element (Utilities|Array|ForEachLoopwithBreak (Variables|/Script/Mordhau.MordhauCharacter|GetEquipment (Class|MordhauPlayerController|GetControlledMordhauCharacter _asbp_mordhau_player_controller false)))
    (:LoopBody
      (bind _asbp_portal_crossbow (Utilities|Casting|CastToBP_PortalCrossbow _array_element))
      (CallFunction|SpawnorPlacePortal _asbp_portal_crossbow (Variables|/RandomWeapon_BattleRoyal/Weapons/PortalCrossbow/BP_PortalCrossbow.BP_PortalCrossbow_C|GetPortalSpawnMode _asbp_portal_crossbow) Transform))))

(event EventBeginPlay
  (|CallParentFunction) ; This node is disabled and will not be called.\nDrag off pins to build functionality.
)

(event Collision|EventActorBeginOverlap
  (params (OtherActor :type Actor%20Object%20Reference))
  (|CallParentFunction OtherActor) ; This node is disabled and will not be called.\nDrag off pins to build functionality.
)

(event EventTick
  (params (DeltaSeconds :type Float%20%28single-precision%29))
  (|CallParentFunction DeltaSeconds) ; This node is disabled and will not be called.\nDrag off pins to build functionality.
)

(event EventOnProjectileHit
  (params (HitLocation :type Vector :default "0, 0, 0") (HitNormal :type Vector :default "0, 0, 0") (BounceForce :type Float%20%28single-precision%29) (Surface :type Byte :default 0) (bHasHitWorld :type Boolean) (bHasStopped :type Boolean))
  (|CallParentFunction HitLocation HitNormal BounceForce Surface bHasHitWorld bHasStopped)
  (CallFunction|PortalShot (Math|Conversions|ToTransform(Vector) HitLocation)))

(fn ConstructionScript
  (|CallParentFunction))

(fn SpawnPortal
  (params (PortalType :type PortalNumber%20Enum :default "NewEnumerator0") (SpawnPosition :type Transform))
  (bind _returnvalue (Game|SpawnActorfromClass (Variables|Default|GetSpawnObject) SpawnPosition "Undefined" 0 0))
  (bind _asbp_special_portal (Utilities|Casting|CastToBP_SpecialPortal _returnvalue))
  (switch Utilities|FlowControl|Switch|SwitchonPortalNumber PortalType
    (:NewEnumerator0
      (Rendering|Material|SetMaterial (Variables|/RandomWeapon_BattleRoyal/Weapons/PortalCrossbow/BP_SpecialPortal.BP_SpecialPortal_C|GetStaticMesh _asbp_special_portal) 0 "/RandomWeapon_BattleRoyal/Weapons/PortalCrossbow/M_FirstPortal.M_FirstPortal"))
    (:NewEnumerator1
      (Rendering|Material|SetMaterial (Variables|/RandomWeapon_BattleRoyal/Weapons/PortalCrossbow/BP_SpecialPortal.BP_SpecialPortal_C|GetStaticMesh _asbp_special_portal) 0 "/RandomWeapon_BattleRoyal/Weapons/PortalCrossbow/M_SecondPortal.M_SecondPortal")))
  (Variables|/RandomWeapon_BattleRoyal/Weapons/PortalCrossbow/BP_SpecialPortal.BP_SpecialPortal_C|SetPortalType _asbp_special_portal PortalType)
  (return _asbp_special_portal))

(fn IsPortalSpawned
  (params (Crossbow :type BP%20Portal%20Crossbow%20Object%20Reference) (PortalType :type PortalNumber%20Enum :default "NewEnumerator0"))
  (Development|PrintString "IsPortalSpawned")
  (Development|PrintString (Utilities|String|EnumtoString PortalType))
  (switch Utilities|FlowControl|Switch|SwitchonPortalNumber PortalType
    (:NewEnumerator0
      (LocalVariables|SetSpawned (Utilities|IsValid (Variables|/RandomWeapon_BattleRoyal/Weapons/PortalCrossbow/BP_PortalCrossbow.BP_PortalCrossbow_C|GetFirstPortal Crossbow))))
    (:NewEnumerator1
      (LocalVariables|SetSpawned (Utilities|IsValid (Variables|/RandomWeapon_BattleRoyal/Weapons/PortalCrossbow/BP_PortalCrossbow.BP_PortalCrossbow_C|GetSecondPortal Crossbow)))))
  (return (LocalVariables|GetSpawned)))

(fn SpawnorPlacePortal
  (params (Crossbow :type BP%20Portal%20Crossbow%20Object%20Reference) (SpawnMode :type PortalNumber%20Enum :default "NewEnumerator0") (Position :type Transform))
  (bind _isspawned (CallFunction|IsPortalSpawned Crossbow SpawnMode))
  (if _isspawned
    (CallFunction|MovePortal Crossbow SpawnMode Position)
    (else
      (bind _portal (CallFunction|SpawnPortal SpawnMode Position))
      (switch Utilities|FlowControl|Switch|SwitchonPortalNumber SpawnMode
        (:NewEnumerator0
          (bind _output_get (Variables|/RandomWeapon_BattleRoyal/Weapons/PortalCrossbow/BP_PortalCrossbow.BP_PortalCrossbow_C|SetFirstPortal Crossbow _portal))
          (Variables|/RandomWeapon_BattleRoyal/Weapons/PortalCrossbow/BP_SpecialPortal.BP_SpecialPortal_C|SetPortalCrossbow _output_get Crossbow)
          (Development|PrintString "First Portal Spawned"))
        (:NewEnumerator1
          (bind _output_get_2 (Variables|/RandomWeapon_BattleRoyal/Weapons/PortalCrossbow/BP_PortalCrossbow.BP_PortalCrossbow_C|SetSecondPortal Crossbow _portal))
          (Variables|/RandomWeapon_BattleRoyal/Weapons/PortalCrossbow/BP_SpecialPortal.BP_SpecialPortal_C|SetPortalCrossbow _output_get_2 Crossbow)
          (Development|PrintString "Second portal spawned")))))
  (return))

(fn MovePortal
  (params (Crossbow :type BP%20Portal%20Crossbow%20Object%20Reference) (PortalType :type PortalNumber%20Enum :default "NewEnumerator0") (MovePosition :type Transform))
  (bind (_location _rotation) (Math|Transform|BreakTransform MovePosition))
  (switch Utilities|FlowControl|Switch|SwitchonPortalNumber PortalType
    (:NewEnumerator0
      (LocalVariables|SetPortal (Variables|/RandomWeapon_BattleRoyal/Weapons/PortalCrossbow/BP_PortalCrossbow.BP_PortalCrossbow_C|GetSecondPortal Crossbow)))
    (:NewEnumerator1
      (LocalVariables|SetPortal (Variables|/RandomWeapon_BattleRoyal/Weapons/PortalCrossbow/BP_PortalCrossbow.BP_PortalCrossbow_C|GetFirstPortal Crossbow))))
  (Transformation|Teleport (LocalVariables|GetPortal) _location _rotation)
  (return))