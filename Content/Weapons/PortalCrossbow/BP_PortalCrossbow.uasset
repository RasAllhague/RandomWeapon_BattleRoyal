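; BP_PortalCrossbow is a Mordhau crossbow weapon Blueprint with a switchable portal spawn mode.
; On Tick, when it belongs to a character controlled by a BP_MordhauPlayerController, it polls the hard-coded T key and flips PortalSpawnMode between First and Second.
; Portal spawning itself is not in this graph, and the construction script only calls its parent.
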(event EventBeginPlay
  (|CallParentFunction) ; This node is disabled and will not be called.\nDrag off pins to build functionality.
)

(event Collision|EventActorBeginOverlap
  (params (OtherActor :type Actor%20Object%20Reference))
  (|CallParentFunction OtherActor) ; This node is disabled and will not be called.\nDrag off pins to build functionality.
)

(event EventTick
  (params (DeltaSeconds :type Float%20%28single-precision%29))
  (|CallParentFunction DeltaSeconds)
  (if (Class|MordhauEquipment|BelongstoCharacter)
    (bind _asbp_mordhau_player_controller (Utilities|Casting|CastToBP_MordhauPlayerController (Pawn|GetController (Class|MordhauEquipment|GetParentCharacter))))
    (if (Game|Player|WasInputKeyJustPressed _asbp_mordhau_player_controller "T")
      (switch Utilities|FlowControl|Switch|SwitchonPortalNumber (Variables|Default|GetPortalSpawnMode)
        (:NewEnumerator0
          (Variables|Default|SetPortalSpawnMode "NewEnumerator1"))
        (:NewEnumerator1
          (Variables|Default|SetPortalSpawnMode "NewEnumerator0"))))))

(fn ConstructionScript
  (|CallParentFunction))