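; BP_SpecialPortal is one end of the portal pair referenced through PortalCrossbow, teleporting characters between the two.
; Overlapping its box moves a BP_MordhauCharacter slightly above the opposite portal, chosen by PortalType, keeping the character's rotation.
; The destination is put on cooldown before the teleport to prevent bouncing back, and both portals re-arm after a short delay.
; Debug strings print on collision and failed casts.
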(event OnComponentBeginOverlap(Box)
  (params (OverlappedComponent :type Primitive%20Component%20Object%20Reference) (OtherActor :type Actor%20Object%20Reference) (OtherComp :type Primitive%20Component%20Object%20Reference) (OtherBodyIndex :type Integer) (bFromSweep :type Boolean) (SweepResult :type Hit%20Result%20Structure%20%28by%20ref%29))
  (bind _portalcrossbow (Variables|Default|GetPortalCrossbow))
  (bind _secondportal (Variables|/RandomWeapon_BattleRoyal/Weapons/PortalCrossbow/BP_PortalCrossbow.BP_PortalCrossbow_C|GetSecondPortal _portalcrossbow))
  (bind _firstportal (Variables|/RandomWeapon_BattleRoyal/Weapons/PortalCrossbow/BP_PortalCrossbow.BP_PortalCrossbow_C|GetFirstPortal _portalcrossbow))
  (if (not (Variables|Default|GetOnCooldown))
    (Development|PrintString "COllision")
    (bind _asbp_mordhau_character (Utilities|Casting|CastToBP_MordhauCharacter OtherActor)
      (:then
        (switch Utilities|FlowControl|Switch|SwitchonPortalNumber (Variables|Default|GetPortalType)
          (:NewEnumerator0
            (Variables|BP_SpecialPortal_C|SetOnCooldown _secondportal true)
            (Transformation|Teleport _asbp_mordhau_character (+ (.Location (Math|Transform|BreakTransform (Transformation|GetActorTransform _secondportal))) "0, 0,10.000000") (.Rotation (Math|Transform|BreakTransform (Transformation|GetActorTransform _asbp_mordhau_character))))
            (Variables|Default|SetOnCooldown true)
            (Utilities|FlowControl|Delay 2.0)
            (Variables|Default|SetOnCooldown false)
            (Variables|BP_SpecialPortal_C|SetOnCooldown _secondportal false))
          (:NewEnumerator1
            (Variables|BP_SpecialPortal_C|SetOnCooldown _firstportal true)
            (Transformation|Teleport _asbp_mordhau_character (+ (.Location (Math|Transform|BreakTransform (Transformation|GetActorTransform _firstportal))) "0, 0,10.000000") (.Rotation (Math|Transform|BreakTransform (Transformation|GetActorTransform _asbp_mordhau_character))))
            (Variables|Default|SetOnCooldown true)
            (Utilities|FlowControl|Delay 2.0)
            (Variables|Default|SetOnCooldown false)
            (Variables|BP_SpecialPortal_C|SetOnCooldown _firstportal false))))
      (:CastFailed
        (Development|PrintString "Cast failed")))))

(event EventBeginPlay)

(event Collision|EventActorBeginOverlap
  (params (OtherActor :type Actor%20Object%20Reference)))

(event EventTick
  (params (DeltaSeconds :type Float%20%28single-precision%29)))

(fn ConstructionScript)