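; BP_JoshuasWaraxe is a war axe weapon Blueprint that adds a stamina cost to attacks made through its parent's FireProjectile logic.
; Its FireProjectile override calls the parent, then deducts a fixed amount of stamina from the owning character, with replication, if the weapon belongs to one.
; All other behavior is inherited, as the construction script only calls its parent and the remaining events are disabled stubs.
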(event EventBeginPlay
  (|CallParentFunction) ; This node is disabled and will not be called.\nDrag off pins to build functionality.
)

(event Collision|EventActorBeginOverlap
  (params (OtherActor :type Actor%20Object%20Reference))
  (|CallParentFunction OtherActor) ; This node is disabled and will not be called.\nDrag off pins to build functionality.
)

(event EventTick
  (params (DeltaSeconds :type Float%20%28single-precision%29))
  (|CallParentFunction DeltaSeconds) ; This node is disabled and will not be called.\nDrag off pins to build functionality.
)

(event EventFireProjectile
  (params (Origin :type Vector%20%28by%20ref%29 :default "0, 0, 0") (Orientation :type Rotator%20%28by%20ref%29 :default "0, 0, 0") (OwningController :type Controller%20Object%20Reference) (ExpectedDelay :type Float%20%28single-precision%29))
  (|CallParentFunction Origin Orientation OwningController ExpectedDelay)
  (if (Class|MordhauEquipment|BelongstoCharacter)
    (Class|MordhauCharacter|OffsetStamina (Class|MordhauEquipment|GetParentCharacter) -15 true)))

(fn ConstructionScript
  (|CallParentFunction))