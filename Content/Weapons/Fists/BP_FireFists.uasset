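; BP_FireFists is a fists weapon variant that sets characters it hits on fire.
; On hit it runs the parent behavior, then starts burning on the struck BP_MordhauCharacter's BurnableComponent using its Duration, Damage and Tick values.
; The wielder's player controller is passed as instigator, so burning only applies when the wielder has a BP_MordhauPlayerController.
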(event EventBeginPlay
  (|CallParentFunction) ; This node is disabled and will not be called.\nDrag off pins to build functionality.
)

(event Collision|EventActorBeginOverlap
  (params (OtherActor :type Actor%20Object%20Reference))
  (|CallParentFunction OtherActor) ; This node is disabled and will not be called.\nDrag off pins to build functionality.
)

(event EventTick
  (params (DeltaSeconds :type Float%20%28single-precision%29))
  (|CallParentFunction DeltaSeconds) ; This node is disabled and will not be called.\nDrag off pins to build functionality.
)

(event EventOnHit
  (params (Actor :type Actor%20Object%20Reference) (Move :type EAttackMove%20Enum :default "RightStrike") (Bone :type Name :default "None") (WorldLocation :type Vector%20%28by%20ref%29 :default "0, 0, 0") (Tier :type Byte :default 0) (SurfaceType :type Byte :default 0))
  (|CallParentFunction Actor Move Bone WorldLocation Tier SurfaceType)
  (bind _asbp_mordhau_character (Utilities|Casting|CastToBP_MordhauCharacter Actor))
  (bind _asbp_mordhau_player_controller (Utilities|Casting|CastToBP_MordhauPlayerController (Pawn|GetController (Class|MordhauEquipment|GetParentCharacter))))
  (Class|BurnableComponent|StartBurning (Variables|/Script/Mordhau.AdvancedCharacter|GetBurnableComponent _asbp_mordhau_character) (Variables|Default|GetDuration) (Variables|Default|GetDamage) (Variables|Default|GetTick) 0 _asbp_mordhau_player_controller))

(fn ConstructionScript
  (|CallParentFunction))