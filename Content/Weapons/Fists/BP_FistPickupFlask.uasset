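; BP_FistPickupFlask is a consumable flask weapon that swaps the holder's fists for a configured FistToEquip class when an attack starts.
; On attack, it scans the character's Equipment for the first BP_FistsWeapon child, force-drops and destroys it.
; It then spawns the new fist weapon and picks it up into the same slot index.
; Finally the flask force-drops and destroys itself, even if no fists were found.
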(event EventBeginPlay
  (|CallParentFunction) ; This node is disabled and will not be called.\nDrag off pins to build functionality.
)

(event Collision|EventActorBeginOverlap
  (params (OtherActor :type Actor%20Object%20Reference))
  (|CallParentFunction OtherActor) ; This node is disabled and will not be called.\nDrag off pins to build functionality.
)

(event EventTick
  (params (DeltaSeconds :type Float%20%28single-precision%29))
  (|CallParentFunction DeltaSeconds) ; This node is disabled and will not be called.\nDrag off pins to build functionality.
)

(event EventOnAttackStarted
  (params (Move :type EAttackMove%20Enum :default "RightStrike") (Angle :type Float%20%28single-precision%29))
  (bind _returnvalue (Class|MordhauEquipment|GetParentCharacter))
  (|CallParentFunction Move Angle)
  (bind (_array_element _array_index) (Utilities|Array|ForEachLoopwithBreak (Variables|/Script/Mordhau.MordhauCharacter|GetEquipment _returnvalue) :!label _label)
    (:LoopBody
      (if (Utilities|ClassIsChildOf (Utilities|GetClass _array_element) "/Game/Mordhau/Blueprints/Equipment/Weapons/BP_FistsWeapon.BP_FistsWeapon_C")
        (bind _returnvalue_2 (Class|MordhauCharacter|DropEquipment _returnvalue _array_element true))
        (Actor|DestroyActor _returnvalue_2)
        (bind _returnvalue_3 (Game|SpawnActorfromClass (Variables|Default|GetFistToEquip) (Math|Transform|MakeTransform "0, 0, 0") "AlwaysSpawn" _returnvalue 0))
        (Class|MordhauCharacter|PickUptoSlot _returnvalue _returnvalue_3 (Math|Conversions|ToByte(Integer) _array_index))
        (goto _label Break)))
    (:Completed
      (bind _returnvalue_4 (Class|MordhauCharacter|DropEquipment _returnvalue self true))
      (Actor|DestroyActor _returnvalue_4))))

(fn ConstructionScript
  (|CallParentFunction))